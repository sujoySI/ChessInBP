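; BP_Board is the chess board actor that sets up an indexed array for the board's squares.
; Initialize calls SetSquaresRef, which runs only while BoardSquaresRef is empty, finding and initializing every BP_BoardSquares actor.
; MakeSquareIndex flattens each square's 1-based X and Y into a zero-based index using BoardWidth.
; The array set grows BoardSquaresRef to that index, but shows no Item input.
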(fn `Initialize`
  (`self.SetSquaresRef`))

(fn `MakeSquareIndex`
  (params (x :type Integer) (y :type Integer))
  (returns (Index :type Integer))
  (return (+ (* (- x 1) (`self.BoardWidth`)) (- y 1))))

(fn `SetSquaresRef`
  (if (== (`KismetArrayLibrary.Array_Length` (`self.BoardSquaresRef`)) 0)
    (bind _outactors (`GameplayStatics.GetAllActorsOfClass` "/Game/Chess/Blueprints/Board/BP_BoardSquares.BP_BoardSquares_C"))
    (for _array_element _outactors
      (`/Game/Chess/Blueprints/Board/BP_BoardSquares.Initialize` _array_element)
      (`KismetArrayLibrary.Array_Set` (`self.BoardSquaresRef`) (`self.MakeSquareIndex` (`/Game/Chess/Blueprints/Board/BP_BoardSquares.X` _array_element) (`/Game/Chess/Blueprints/Board/BP_BoardSquares.Y` _array_element)) null true))))

(fn `UserConstructionScript`)